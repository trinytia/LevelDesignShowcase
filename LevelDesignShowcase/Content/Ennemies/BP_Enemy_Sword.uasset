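; Sword enemy Blueprint that chases the player and strikes in melee.
; While alive, seeing the player and not attacking, Tick runs AI MoveTo toward PlayerRef.
; On arrival, a DoOnce-gated attack waits briefly, then sphere-traces forward from the capsule on the Camera channel with debug drawing.
; Only a hit on BP_ThirdPersonCharacter deals damage, clears Attack and, after a short cooldown, resets the gate.
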(event Custom|Reset
  (bind _capsulecomponent (Variables|Default|GetCapsuleComponent))
  (bind _returnvalue (Transformation|GetWorldLocation _capsulecomponent))
  (Utilities|FlowControl|DoOnce false) ; enters at Reset
)

(event EventBeginPlay
  (|CallParentFunction) ; This node is disabled and will not be called.\nDrag off pins to build functionality.
)

(event Collision|EventActorBeginOverlap
  (params (OtherActor :type Actor%20Object%20Reference))
  (|CallParentFunction OtherActor) ; This node is disabled and will not be called.\nDrag off pins to build functionality.
)

(event EventTick
  (params (DeltaSeconds :type Float%20%28single-precision%29))
  (bind _capsulecomponent (Variables|Default|GetCapsuleComponent))
  (bind _returnvalue (Transformation|GetWorldLocation _capsulecomponent))
  (|CallParentFunction DeltaSeconds)
  (if (not (Variables|Default|GetDead))
    (if (Variables|Default|GetSeePlayer)
      (if (not (Variables|Default|GetAttack?))
        (AI|AIMoveTo self "0, 0, 0" (Variables|Default|GetPlayer_Ref) 125.0 false
          (:OnSuccess
            (Utilities|FlowControl|DoOnce false
              (:Completed
                (Variables|Default|SetAttack? true)
                (Utilities|FlowControl|Delay 0.8)
                (if (not (Variables|Default|GetDead))
                  (bind _outhit (Collision|SphereTraceByChannel _returnvalue (+ _returnvalue (* (Math|Vector|GetForwardVector _capsulecomponent) 1.5e+02)) 75.0 "TraceTypeQuery2" false 0 "ForDuration"))
                  (bind _asbp_third_person_character (Utilities|Casting|CastToBP_ThirdPersonCharacter (.HitActor (Collision|BreakHitResult _outhit)))
                    (:then
                      (Default|TakeDamages _asbp_third_person_character (Variables|Default|GetDamages)))
                    (:CastFailed
                      _))
                  (Variables|Default|SetAttack? false)
                  (Utilities|FlowControl|Delay 0.5)
                  (CallFunction|Reset))))))))))

(fn ConstructionScript
  (|CallParentFunction))