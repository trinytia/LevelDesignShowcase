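; BP_Enemy is an enemy character that detects the player and can take damage and die.
; Each tick while alive, it sets SeePlayer within VisionRange; non-archers also need a line trace hitting the player.
; SeePlayer clears only out of range with ShouldStopSee enabled.
; TakeDamages reduces Health until Die halts movement and ignores Pawn collision, and the construction script previews the vision sphere.
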(event Custom|DebugRange
  (Rendering|Debug|DrawDebugSphere (Transformation|GetWorldLocation (Variables|Collision|GetCapsuleComponent)) (Variables|Stats|GetVisionRange) 24 "(R=1.000000,G=0.000000,B=0.000000,A=1.000000)" 1.0 1e+01))

(event Custom|Die
  (Components|Movement|StopMovementImmediately (Variables|Character|GetCharacterMovement))
  (Variables|Default|SetDead true)
  (Collision|SetCollisionResponsetoChannel (Variables|Collision|GetCapsuleComponent) "ECC_Pawn" "ECR_Ignore")
  (Variables|/Script/Engine.CharacterMovementComponent|SetMaxWalkSpeed (Variables|Character|GetCharacterMovement) 0.0))

(event EventBeginPlay
  (bind _returnvalue (Actor|GetActorOfClass "/Game/ThirdPerson/Blueprints/BP_ThirdPersonCharacter.BP_ThirdPersonCharacter_C"))
  (Variables|Default|SetPlayer_Ref _returnvalue)
  (Variables|/Script/Engine.CharacterMovementComponent|SetMaxWalkSpeed (Variables|Character|GetCharacterMovement) (Variables|Stats|GetSpeed)))

(event EventTick
  (params (DeltaSeconds :type Float%20%28single-precision%29))
  (bind _returnvalue (Transformation|GetActorLocation))
  (bind _player_ref (Variables|Default|GetPlayer_Ref))
  (bind _returnvalue_2 (Transformation|GetActorLocation _player_ref))
  (if (not (Variables|Default|GetDead))
    (if (<= (Math|Vector|Distance(Vector) _returnvalue _returnvalue_2) (Variables|Stats|GetVisionRange))
      (if (Variables|Default|GetArcher)
        _
        (else
          (bind _outhit (Collision|LineTraceByChannel _returnvalue _returnvalue_2 "TraceTypeQuery2" false 0 "None"))
          (Utilities|Casting|CastToBP_ThirdPersonCharacter (.HitActor (Collision|BreakHitResult _outhit)))))
      (Variables|Default|SetSeePlayer true)
      (elif (Variables|Default|GetShouldStopSee?)
        (Variables|Default|SetSeePlayer false)))))

(event EventTakeDamages
  (params (Damages :type Integer))
  (bind _output_get (Variables|Default|SetHealth (- (Variables|Default|GetHealth) Damages)))
  (if (<= _output_get 0)
    (CallFunction|Die)))

(fn ConstructionScript
  (CallFunction|DebugRange))