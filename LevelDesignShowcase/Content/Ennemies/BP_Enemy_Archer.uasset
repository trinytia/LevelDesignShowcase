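; Archer enemy that makes timed hitscan shots at the player.
; While it sees the player and lives, Tick turns it toward them and a DoOnce starts each attack, setting the Attack flag.
; After a wind-up delay, a line trace to the player's current position drives a Niagara arrow effect, impact sound and damage to any player character hit.
; A short cooldown then resets the DoOnce.
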(event Custom|Reset
  (bind _returnvalue (Transformation|GetActorLocation))
  (Utilities|FlowControl|DoOnce false) ; enters at Reset
)

(event EventBeginPlay
  (|CallParentFunction) ; This node is disabled and will not be called.\nDrag off pins to build functionality.
)

(event Collision|EventActorBeginOverlap
  (params (OtherActor :type Actor%20Object%20Reference))
  (|CallParentFunction OtherActor) ; This node is disabled and will not be called.\nDrag off pins to build functionality.
)

(event EventTick
  (params (DeltaSeconds :type Float%20%28single-precision%29))
  (bind _returnvalue (Transformation|GetActorLocation))
  (|CallParentFunction DeltaSeconds)
  (if (Variables|Default|GetSeePlayer)
    (if (not (Variables|Default|GetDead))
      (Transformation|SetActorRotation (Math|Rotator|FindLookatRotation (Transformation|GetActorLocation) (Transformation|GetActorLocation (Variables|Default|GetPlayer_Ref))))
      (Utilities|FlowControl|DoOnce false
        (:Completed
          (Variables|Default|SetAttack? true)
          (Utilities|FlowControl|Delay 2.0)
          (if (not (Variables|Default|GetDead))
            (bind _outhit (Collision|LineTraceByChannel _returnvalue (Transformation|GetActorLocation (Variables|Default|GetPlayer_Ref)) "TraceTypeQuery2" false 0 "None"))
            (bind _returnvalue_2 (Niagara|SpawnSystematLocation "/Game/VFX/NS_Arrow.NS_Arrow" _returnvalue))
            (Effects|Components|ParticleSystem|SetVectorParameter _returnvalue_2 "End_Loc" (.Location (Collision|BreakHitResult _outhit)))
            (Effects|Components|ParticleSystem|SetColorParameter _returnvalue_2 "Color" "(R=10.000000,G=0.000000,B=0.000000,A=1.000000)")
            (Effects|Components|ParticleSystem|SetFloatParameter _returnvalue_2 "Size" 1e+01)
            (Audio|PlaySoundatLocation "/Game/Ennemies/Archer/Impact_Cue.Impact_Cue" (.Location (Collision|BreakHitResult _outhit)) "0, 0, 0" 1.0 1.0 0.0 "/Game/Ennemies/Archer/SA_Generic.SA_Generic" 0 0 0)
            (bind _asbp_third_person_character (Utilities|Casting|CastToBP_ThirdPersonCharacter (.HitActor (Collision|BreakHitResult _outhit)))
              (:then
                (Default|TakeDamages _asbp_third_person_character (Variables|Default|GetDamages)))
              (:CastFailed
                _))
            (Variables|Default|SetAttack? false)
            (Utilities|FlowControl|Delay 0.5)
            (CallFunction|Reset)))))))

(fn ConstructionScript
  (|CallParentFunction))